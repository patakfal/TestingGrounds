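; AI controller for guard NPCs that spots non-friendly actors and makes the controlled character aim and shoot.
; On BeginPlay it loads the PatrolData blackboard and runs the GuardBehaviour behavior tree.
; Perception updates write sensed actors lacking the "Friendly" tag to the enemy key and clear it when one is lost.
; Every tick it sets the character's Aiming and Shooting flags from whether a focus actor exists.
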(event `self.ReceiveTick`
  (params (DeltaSeconds :type "Float (single-precision)"))
  (bind _returnvalue (`KismetSystemLibrary.IsValid` (`self.GetFocusActor`)))
  ;[1 1 1] Setting Amining when in Focus
  (bind _ascharacter (cast `/Game/Dynamic/Character/Behaviour/Character` (`self.K2_GetPawn`)))
  (set `/Game/Dynamic/Character/Behaviour/Character.Aiming` _returnvalue _ascharacter)
  (set `/Game/Dynamic/Character/Behaviour/Character.Shooting` _returnvalue _ascharacter))

(event `self.ReceiveBeginPlay`
  (bind _blackboardcomponent (`self.UseBlackboard` "/Game/Dynamic/Character/AI/PatrolData.PatrolData"))
  (`self.RunBehaviorTree` "/Game/Dynamic/Character/AI/GuardBehaviour.GuardBehaviour")
  (set `self.BlackBoardComp` _blackboardcomponent))

(event `self.AIPerception.OnTargetPerceptionUpdated`
  (params (Actor :type "Actor Object Reference") (Stimulus :type "AIStimulus Structure"))
  (bind _blackboardcomp (`self.BlackBoardComp`))
  (bind _enemykey (`self.EnemyKey`))
  (if (`self.ActorHasTag` Actor "Friendly")
    _
    (elif (`.bSuccessfullySensed` (break `AIStimulus` Stimulus))
      (`BlackboardComponent.SetValueAsObject` _blackboardcomp _enemykey Actor)
      (else
        (`BlackboardComponent.ClearValue` _blackboardcomp _enemykey)))))

(fn `UserConstructionScript`)